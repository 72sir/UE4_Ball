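; Game instance that holds level progression in LvlData: each level's availability and three completion-path flags (Ways).
; UpdateLvlData ORs the given way into that level's flags via MergeWays, then marks the next level available while keeping its existing ways.
; SaveGame and LoadGame copy LvlData to and from a B_Save object in a single save slot, separately from updates.
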(event `UpdateLvlData`
  (params (Level :type Integer) (Way :type Integer))
  (bind _returnvalue (+ Level 1))
  ;[1 1 1] Update Level Data
  (`self.SetLevelData` Level true (`self.MergeWays` Way (`.Ways` (`self.GetLvlData` Level)))
    (:`  `
      (if (< _returnvalue (`KismetArrayLibrary.Array_Length` (`.LevelsData_3_941C0FC141523BBEF603D4AB0D4AFE30` (break `/Game/Blueprints/St_LvlData` (`self.LvlData`)))))
        (`self.SetLevelData` _returnvalue true (`.Ways` (`self.GetLvlData` _returnvalue)))))))

(event `SaveGame`
  ;[1 1 1] SaveGame
  (bind _returnvalue (`GameplayStatics.CreateSaveGameObject` "/Game/Blueprints/B_Save.B_Save_C"))
  (bind _asb_save (cast `/Game/Blueprints/B_Save` _returnvalue))
  (set `/Game/Blueprints/B_Save.LvlData` (`self.LvlData`) _asb_save)
  (`GameplayStatics.SaveGameToSlot` _returnvalue "SaveGame"))

(event `LoadGame`
  ;[1 1 1] LoadGame
  (bind _returnvalue (`GameplayStatics.LoadGameFromSlot` "SaveGame"))
  (bind _asb_save (cast `/Game/Blueprints/B_Save` _returnvalue))
  (set `self.LvlData` (`/Game/Blueprints/B_Save.LvlData` _asb_save)))