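; Touch-controlled pawn that either rotates the view by dragging or holds and launches a Ball.
; On press, a TouchBall check chooses between starting a camera drag and flagging the Ball as held.
; While a drag keeps the Tick gate open, horizontal finger offset from the start point sets the pawn's yaw.
; Release launches a held Ball and closes the gate.
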(event `self.ReceiveTick`
  (params (DeltaSeconds :type "Float (single-precision)"))
  ;[1 1 1] Движение камеры
  (`/Engine/EditorBlueprintResources/StandardMacros.Gate` true :!label _label
    (:`Exit`
      (`self.moveCamera`))))

(event `InputTouch`
  (params (Location :type "Vector Structure") (FingerIndex :type "ETouchIndex Enum"))
  ;[1 1 1] Движение камеры
  (:`Pressed`
    (`|ExecutionSequence`
      (:`then_1`
        (if (!= (`self.touchBall`) (`self.Ball`))
          (`self.initCameraRot` Location
            (:`Open`
              (goto _label :!via `Open`)))
          (else
            (`self.ballMove` :!label _label_2))))))
  (:`Released`
    (`|ExecutionSequence`
      (:`then_0`
        (goto _label_2 :!via `Unpressed`))
      (:`then_1`
        (goto _label :!via `Close`)))))

(fn `UserConstructionScript`)