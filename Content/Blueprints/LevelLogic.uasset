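; Level logic for a ball level with three alternative routes, recording which route the ball takes to the finish.
; Each route has paired overlap triggers gated by a Ways macro to set Way, while entering one toggles Spawner actors for its exit and other routes.
; Finish saves level and route through the game instance, then calls Restart to reset ball and routes.
; Tick moves the pawn after the launched ball within clamped camera bounds.
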(event `self.ReceiveBeginPlay`
  ;[1 1 1] BeginPlay
  (`|ExecutionSequence`
    (:`then_0`
      (bind _asball (cast `/Game/Models/ball` (`self.Ball`)))
      (set `self.CurBall` _asball)
      (`self.K2_SetActorLocation` (`GameplayStatics.GetPlayerPawn` 0) (`SceneComponent.K2_GetComponentLocation` (`/Game/Models/ball.DefaultSceneRoot` _asball)) false false)
      (bind _asgm_bounce (cast `/Game/Blueprints/GM_Bounce` (`GameplayStatics.GetGameMode`)))
      (add `/Game/Blueprints/GM_Bounce.RestartLevel` _asgm_bounce (delegate `Restart`))
      (bind _aspawn_sir (cast `/Game/Blueprints/Pawn_sir` (`GameplayStatics.GetPlayerPawn` 0)))
      (set `/Game/Blueprints/Pawn_sir.Ball` (`self.CurBall`) _aspawn_sir))
    (:`then_1`
      (`self.Spawner` (`self.actWay1-2`)
        (:` `
          (`self.Spawner` (`self.actWay2-2`)
            (:` `
              (`self.Spawner` (`self.actWay3-2`)))))))))

(event `Restart`
  (bind _curball (`self.CurBall`))
  (bind _inlocation (`/Game/Models/ball.InLocation` _curball))
  (bind _ball_sir (`/Game/Models/ball.Ball_sir` _curball))
  ;[1 1 1] BeginPlay
  (set `/Game/Models/ball.hit` true (stale `self.ReceiveBeginPlay` _asball))
  (set `self.way` -1)
  (`SceneComponent.K2_SetWorldLocation` _ball_sir _inlocation false false)
  (`PrimitiveComponent.SetSimulatePhysics` _ball_sir false)
  (set `/Game/Models/ball.Launched` false _curball)
  (`self.K2_SetActorLocation` (`GameplayStatics.GetPlayerPawn` 0) _inlocation false false)
  (`|ExecutionSequence`
    (:`then_0`
      (if (`self.bWay1-2`)
        (`self.Spawner` (`self.actWay1-2`))))
    (:`then_1`
      (if (not (`self.bWay1-1`))
        (`self.Spawner` (`self.actWay1-1`))))
    (:`then_2`
      (if (`self.bWay2-2`)
        (`self.Spawner` (`self.actWay2-2`))))
    (:`then_3`
      (if (not (`self.bWay2-1`))
        (`self.Spawner` (`self.actWay2-1`))))
    (:`then_4`
      (if (`self.bWay3-2`)
        (`self.Spawner` (`self.actWay3-2`))))
    (:`then_5`
      (if (not (`self.bWay3-1`))
        (`self.Spawner` (`self.actWay3-1`))))
    (:`then_6`
      (`self.DefaultValueVariables`))))

(event `self.Finish.OnActorBeginOverlap`
  (params (OverlappedActor :type "Actor Object Reference") (OtherActor :type "Actor Object Reference"))
  ;[1 1 1] Finish
  (`KismetSystemLibrary.PrintString` (`KismetStringLibrary.Conv_IntToString` (`self.way`)) true true (struct :`A` 1.0))
  (bind _asgm_instanse (cast `/Game/Blueprints/Gm_instanse` (`GameplayStatics.GetGameInstance`)))
  (`/Game/Blueprints/Gm_instanse.UpdateLvlData` _asgm_instanse (`self.Level`) (`self.way`))
  (`/Game/Blueprints/Gm_instanse.SaveGame` _asgm_instanse)
  (`self.Restart`))

(event `self.ReceiveTick`
  (params (DeltaSeconds :type "Float (single-precision)"))
  (`self.CameraMover`))

(event `self.actWay1-1.OnActorBeginOverlap`
  (params (OverlappedActor :type "Actor Object Reference") (OtherActor :type "Actor Object Reference"))
  (`self.Ways` :!label _label
    (:`Out`
      (set `self.way` 0))))

(event `self.actWay1-2.OnActorBeginOverlap`
  (params (OverlappedActor :type "Actor Object Reference") (OtherActor :type "Actor Object Reference"))
  (goto _label :!via `2`))

(event `self.actWay1-1.OnActorBeginOverlap`
  (params (OverlappedActor :type "Actor Object Reference") (OtherActor :type "Actor Object Reference"))
  ;[1 1 1] Путь 1
  (if (`self.bWay1-1`)
    (set `self.bWay1-1` false)
    (set `self.bWay1-2` true)
    (`self.Spawner` (`self.actWay1-2`)
      (:` `
        (`self.CheckWayHiddenOtherActor` (`self.actWay1-1`)
          (:`  `
            (`self.Ways` :!label _label_2
              (:`Out`
                (set `self.way` 0)))))))))

(event `self.actWay2-1.OnActorBeginOverlap`
  (params (OverlappedActor :type "Actor Object Reference") (OtherActor :type "Actor Object Reference"))
  (`self.Ways` :!label _label_3
    (:`Out`
      (set `self.way` 1))))

(event `self.actWay1-2.OnActorBeginOverlap`
  (params (OverlappedActor :type "Actor Object Reference") (OtherActor :type "Actor Object Reference"))
  ;[1 1 1] Путь 1
  (set `self.bWay1-2` false)
  (goto _label_2 :!via `2`))

(event `self.Way2-2.OnActorBeginOverlap`
  (params (OverlappedActor :type "Actor Object Reference") (OtherActor :type "Actor Object Reference"))
  (goto _label_3 :!via `2`))

(event `self.actWay2-1.OnActorBeginOverlap`
  (params (OverlappedActor :type "Actor Object Reference") (OtherActor :type "Actor Object Reference"))
  ;[1 1 1] Путь 2
  (if (`self.bWay2-1`)
    (set `self.bWay2-1` false)
    (set `self.bWay2-2` true)
    (`self.Spawner` (`self.actWay2-2`)
      (:` `
        (`self.CheckWayHiddenOtherActor` (`self.actWay2-1`)
          (:`  `
            (`self.Ways` :!label _label_4
              (:`Out`
                (set `self.way` 1)))))))))

(event `self.Way3-1.OnActorBeginOverlap`
  (params (OverlappedActor :type "Actor Object Reference") (OtherActor :type "Actor Object Reference"))
  (`self.Ways` :!label _label_5
    (:`Out`
      (set `self.way` 2))))

(event `self.actWay2-2.OnActorBeginOverlap`
  (params (OverlappedActor :type "Actor Object Reference") (OtherActor :type "Actor Object Reference"))
  ;[1 1 1] Путь 2
  (set `self.bWay2-2` false)
  (goto _label_4 :!via `2`))

(event `self.Way3-2.OnActorBeginOverlap`
  (params (OverlappedActor :type "Actor Object Reference") (OtherActor :type "Actor Object Reference"))
  (goto _label_5 :!via `2`))

(event `self.actWay3-1.OnActorBeginOverlap`
  (params (OverlappedActor :type "Actor Object Reference") (OtherActor :type "Actor Object Reference"))
  ;[1 1 1] путь - 3
  (if (`self.bWay3-1`)
    (set `self.bWay3-1` false)
    (set `self.bWay3-2` true)
    (`self.Spawner` (`self.actWay3-2`)
      (:` `
        (`self.CheckWayHiddenOtherActor` (`self.actWay3-1`)
          (:`  `
            (`self.Ways` :!label _label_6
              (:`Out`
                (set `self.way` 2)))))))))

(event `self.actWay3-2.OnActorBeginOverlap`
  (params (OverlappedActor :type "Actor Object Reference") (OtherActor :type "Actor Object Reference"))
  ;[1 1 1] путь - 3
  (set `self.bWay3-2` false)
  (goto _label_6 :!via `2`))

(fn `CameraMover`
  (bind _curball (`self.CurBall`))
  (if (`/Game/Models/ball.Launched` _curball)
    (`self.K2_SetActorLocation` (`GameplayStatics.GetPlayerPawn` 0) (`self.ClampVector` (`self.CamVec1`) (`self.CamVec2`) (`SceneComponent.K2_GetComponentLocation` (`/Game/Models/ball.Ball_sir` _curball))) false false)))

(fn `UserConstructionScript`)