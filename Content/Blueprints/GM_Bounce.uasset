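; Game mode for the Bounce game that sets up the in-game UI and handles pausing and level restarts.
; On BeginPlay it loads the saved game through Gm_instanse, shows the mouse cursor, adds Play and Restart buttons via a CreateButton helper, and pre-creates the Pause and LevelSelect widgets.
; Pause swaps the buttons with the pause widget and sets the game's paused state.
; Restart unpauses, then calls CallRestartLevel.
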(event `self.ReceiveBeginPlay`
  ;[1 1 1] Begin
  (`|ExecutionSequence`
    (:`then_0`
      (bind _asgm_instanse (cast `/Game/Blueprints/Gm_instanse` (`GameplayStatics.GetGameInstance`)))
      (`/Game/Blueprints/Gm_instanse.LoadGame` _asgm_instanse))
    (:`then_1`
      (bind _out (`self.CreateButton` "/Game/UI/Play.Play_C" (150.0 40.0) (20.0 20.0)))
      (set `self.W_Play` _out)
      (bind _returnvalue (`|CreateWidget` "/Game/UI/Pause.Pause_C" (`GameplayStatics.GetPlayerController` 0)))
      (set `self.W_Pause` _returnvalue)
      (`UserWidget.AddToViewport` (`self.W_Play`) 0)
      (bind _out_2 (`self.CreateButton` "/Game/UI/Restart.Restart_C" (150.0 40.0) (20.0 80.0)))
      (set `self.W_Pausebtn` _out_2)
      (`UserWidget.AddToViewport` _out_2 0)
      (bind _returnvalue_2 (`|CreateWidget` "/Game/UI/LevelSelect.LevelSelect_C" (`GameplayStatics.GetPlayerController` 0)))
      (set `self.W_LvlSel` _returnvalue_2))
    (:`then_2`
      (set `PlayerController.bShowMouseCursor` true (`GameplayStatics.GetPlayerController` 0)))))

(event `Pause`
  (params (Pause :type Boolean))
  (bind _w_pausebtn (`self.W_Pausebtn`))
  ;[1 1 1] Pause
  (if Pause
    (`UserWidget.AddToViewport` (`self.W_Pause`) 0)
    (`Widget.RemoveFromParent` _w_pausebtn)
    (`Widget.RemoveFromParent` (`self.W_Play`))
    (else
      (`UserWidget.AddToViewport` (`self.W_Play`) 0)
      (`UserWidget.AddToViewport` _w_pausebtn 0)
      (`Widget.RemoveFromParent` (`self.W_Pause`))))
  (`GameplayStatics.SetGamePaused` Pause))

(event `Restart`
  ;[1 1 1] Restart
  (`self.Pause` false)
  (`self.RestartLevel`))

(fn `CreateButton`
  (params (Button :type "UserWidget Class Reference") (Size :type "Vector2D Structure") (Position :type "Vector2D Structure"))
  (returns (Out :type "UserWidget Object Reference"))
  ;[1 1 1] Создание кнопки
  (bind _returnvalue (`|CreateWidget` Button (`GameplayStatics.GetPlayerController` 0)))
  (`UserWidget.SetDesiredSizeInViewport` _returnvalue Size)
  (`UserWidget.SetPositionInViewport` _returnvalue Position true)
  (return _returnvalue))

(fn `UserConstructionScript`)